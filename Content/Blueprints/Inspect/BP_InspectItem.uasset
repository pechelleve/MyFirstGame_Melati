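; BP_InspectItem is an actor that presents an item for inspection, showing its mesh alongside a name and description.
; The Inspect event stores the character, sets the mesh, adds a W_Inspect widget to the viewport and toggles player input.
; Pressing IA_Interact toggles input again, then removes the widget and destroys the actor if that widget is valid.
; Its Interact function is a stub that returns false.
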(event Input|EnhancedActionEvents|EnhancedInputActionIA_Interact
  (params (ActionValue :type Boolean) (ElapsedSeconds :type Float%20%28double-precision%29) (TriggeredSeconds :type Float%20%28double-precision%29) (InputAction :type Input%20Action%20Object%20Reference :default "/Game/Input/Actions/IA_Interact.IA_Interact"))
  (bind _returnvalue (Game|GetPlayerController 0))
  (:Started
    (Input|DisableInput _returnvalue)
    (Input|EnableInput _returnvalue)
    (Utilities|IsValid (Variables|Default|GetInspectWidget%20Reference)
      (:Is%20Valid
        (Widget|RemovefromParent (Variables|Default|GetInspectWidget%20Reference))
        (Variables|Default|SetInspectWidget%20Reference 0)
        (Actor|DestroyActor)))))

(event EventInspect
  (params (Character :type BP%20Third%20Person%20Character%20Object%20Reference) (Inspected%20Item :type Static%20Mesh%20Object%20Reference) (Item%20Name :type Text) (Item%20Description :type Text))
  (bind _returnvalue (Game|GetPlayerController 0))
  (Variables|Default|SetCharacter Character)
  (Components|StaticMesh|SetStaticMesh (Variables|Default|GetItem) Inspected%20Item)
  (bind _returnvalue_2 (UserInterface|CreateWidget "/Game/Blueprints/Inspect/W_Inspect.W_Inspect_C" 0 Item%20Name Item%20Description))
  (bind _output_get (Variables|Default|SetInspectWidget%20Reference _returnvalue_2))
  (UserInterface|Viewport|AddtoViewport _output_get 0)
  (Input|DisableInput _returnvalue)
  (Input|EnableInput _returnvalue))

(fn ConstructionScript)

(fn Interact
  (params (Interactor :type Character%20Object%20Reference))
  (return false))